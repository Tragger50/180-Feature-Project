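; Player character with camera-relative movement, jump, lock-on targeting and posture-based combat that hands deflect and attack input to a combat component.
; Lock-on capsule-traces from the camera for an actor with AC_Lockon, then each tick turns camera and player toward it, blocking look input.
; Posture recovers each tick via negative damage, scaled by health and blocking.
; Death disables movement; posture break does until its montage completes.
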(event OnDeath(AC_Health_Posture)
  ;[0 0 0 0.5 32] AC_Health_Posture
  ;;[0.15 0.15 0.15 0.5] On Player death
  (Variables|Default|SetCanMove false)
  (Development|PrintString "Dead" true true "(R=0.789814,G=0.893905,B=1.000000,A=1.000000)" 6.0))

(event OnPostureBreak(AC_Health_Posture)
  ;[0 0 0 0.5 32] AC_Health_Posture
  ;;[0.15 0.15 0.15 0.5] On Posture Break
  (Variables|Default|SetCanMove false)
  (Animation|Montage|PlayMontage (Variables|Character|GetMesh) "/Game/Animations/AM_Parry.AM_Parry"
    (:OnCompleted
      (Variables|Default|SetCanMove true)
      (Variables|/Game/Blueprints/ActorComponents/AC_Health_Posture.AC_Health_Posture_C|SetCurrentPosture (Variables|Default|GetAC_Health_Posture) 0.0))))

(event Custom|CameraLockCheck
  (params (Delta%20Time :type Float%20%28double-precision%29))
  ;[0 0 0 0.5 32] Camera
  ;;[0.15 0.15 0.15 0.5] Lock the camera to target
  (if (Variables|Default|GetCameraLocked)
    (CallFunction|CameraLock Delta%20Time (Variables|/Game/Blueprints/ActorComponents/AC_Lockon.AC_Lockon_C|GetStoreVectorSpotLockOn (Actor|GetComponentbyClass (Variables|Default|GetLockOnActor) "/Game/Blueprints/ActorComponents/AC_Lockon.AC_Lockon_C")))))

(event Input|EnhancedActionEvents|EnhancedInputActionIA_Move
  (params (ActionValue :type Vector%202D%20Structure) (ElapsedSeconds :type Float%20%28double-precision%29) (TriggeredSeconds :type Float%20%28double-precision%29) (InputAction :type Input%20Action%20Object%20Reference :default "/Game/Input/IA_Move.IA_Move"))
  (bind _returnvalue (Math|Vector2D|Normalize2D ActionValue))
  (bind _returnvalue_2 (Pawn|GetControlRotation :!class /Script/Engine.Pawn))
  ;[0 0 0 0.5 32] Movement
  ;;[0.15 0.15 0.15 0.5] Move Player (Needs to be in BP_Player to access camera easily)
  (if (Variables|Default|GetCanMove)
    (Utilities|FlowControl|Sequence
      (:then_0
        ;;;[0.15 0.15 0.15 0.5] Move WS
        (Pawn|Input|AddMovementInput (Math|Vector|GetRightVector (Math|Rotator|MakeRotator (.roll _returnvalue_2) 0.0 (.yaw _returnvalue_2))) (.x _returnvalue) false))
      (:then_1
        ;;;[0.15 0.15 0.15 0.5] Move AD
        (Pawn|Input|AddMovementInput (Math|Vector|GetForwardVector (Math|Rotator|MakeRotator 0.0 0.0 (.yaw (Pawn|GetControlRotation :!class /Script/Engine.Pawn)))) (.y _returnvalue) false)))))

(event Input|EnhancedActionEvents|EnhancedInputActionIA_Look
  (params (ActionValue :type Vector%202D%20Structure) (ElapsedSeconds :type Float%20%28double-precision%29) (TriggeredSeconds :type Float%20%28double-precision%29) (InputAction :type Input%20Action%20Object%20Reference :default "/Game/Input/IA_Look.IA_Look"))
  ;[0 0 0 0.5 32] Camera
  ;;[0.15 0.15 0.15 0.5] Rotate Camera
  ;;;[0.15 0.15 0.15 0.5] prevent camera rotation by the player while locked on
  (if (not (Variables|Default|GetCameraLocked))
    (Pawn|Input|AddControllerYawInput (.x ActionValue))
    (Pawn|Input|AddControllerPitchInput (.y ActionValue))))

(event Input|EnhancedActionEvents|EnhancedInputActionIA_Jump
  (params (ActionValue :type Boolean) (ElapsedSeconds :type Float%20%28double-precision%29) (TriggeredSeconds :type Float%20%28double-precision%29) (InputAction :type Input%20Action%20Object%20Reference :default "/Game/Input/IA_Jump.IA_Jump"))
  ;[0 0 0 0.5 32] Movement
  ;;[0.15 0.15 0.15 0.5] jump, max jumps set in the bp_player(Self)
  (:Started
    (Character|Jump))
  (:Completed
    (Character|StopJumping)))

(event Input|EnhancedActionEvents|EnhancedInputActionIA_CameraLock
  (params (ActionValue :type Boolean) (ElapsedSeconds :type Float%20%28double-precision%29) (TriggeredSeconds :type Float%20%28double-precision%29) (InputAction :type Input%20Action%20Object%20Reference :default "/Game/Input/IA_CameraLock.IA_CameraLock"))
  ;[0 0 0 0.5 32] Camera
  ;;[0.15 0.15 0.15 0.5] Lock and Unlock the camera on Middle mouse
  (if (Variables|Default|GetCameraLocked)
    (Variables|Default|SetLockOnTarget "0, 0, 0")
    (Variables|Default|SetCameraLocked false)
    ;;;[0.15 0.15 0.15 0.5] Set Visible Lockon Ui ON/OFF
    (bind _lockonactor (Variables|Default|GetLockOnActor)
      (:then
        (Variables|/Game/Blueprints/ActorComponents/AC_Lockon.AC_Lockon_C|SetWidgetVisiblility (Actor|GetComponentbyClass _lockonactor "/Game/Blueprints/ActorComponents/AC_Lockon.AC_Lockon_C") false))
      (:else))
    (else
      (|CameraTrace(CollapsedGraph))
      (bind _lockonactor_2 (Variables|Default|GetLockOnActor)
        (:then
          (Variables|/Game/Blueprints/ActorComponents/AC_Lockon.AC_Lockon_C|SetWidgetVisiblility (Actor|GetComponentbyClass _lockonactor_2 "/Game/Blueprints/ActorComponents/AC_Lockon.AC_Lockon_C") true))
        (:else)))))

(event Input|EnhancedActionEvents|EnhancedInputActionIA_Deflect
  (params (ActionValue :type Boolean) (ElapsedSeconds :type Float%20%28double-precision%29) (TriggeredSeconds :type Float%20%28double-precision%29) (InputAction :type Input%20Action%20Object%20Reference :default "/Game/Input/IA_Deflect.IA_Deflect"))
  ;[0 0 0 0.5 32] Combat
  (Development|PrintString "Deflect")
  (Default|TriggerSimpleHit (Variables|Default|GetAC_CombatSystem)))

(event Input|EnhancedActionEvents|EnhancedInputActionIA_Attack
  (params (ActionValue :type Boolean) (ElapsedSeconds :type Float%20%28double-precision%29) (TriggeredSeconds :type Float%20%28double-precision%29) (InputAction :type Input%20Action%20Object%20Reference :default "/Game/Input/IA_Attack.IA_Attack"))
  ;[0 0 0 0.5 32] Combat
  (Development|PrintString "Attack")
  (Default|TriggerAdvancedHit (Variables|Default|GetAC_CombatSystem)))

(event Input|EnhancedActionEvents|EnhancedInputActionIA_Dash
  (params (ActionValue :type Boolean) (ElapsedSeconds :type Float%20%28double-precision%29) (TriggeredSeconds :type Float%20%28double-precision%29) (InputAction :type Input%20Action%20Object%20Reference :default "/Game/Input/IA_Dash.IA_Dash"))
  ;[0 0 0 0.5 32] Combat
)

(event EventBeginPlay
  ;[0.15 0.15 0.15 0.5] draw hud to screen
  (bind _returnvalue (UserInterface|CreateWidget "/Game/Blueprints/Ui/BP_Hud.BP_Hud_C"))
  (UserInterface|Viewport|AddtoViewport _returnvalue 0))

(event Collision|EventActorBeginOverlap
  (params (OtherActor :type Actor%20Object%20Reference)))

(event EventTick
  (params (DeltaSeconds :type Float%20%28single-precision%29))
  (CallFunction|CameraLockCheck DeltaSeconds)
  (CallFunction|DecreasePosture DeltaSeconds))

(event Input|KeyboardEvents|1
  (params (Key :type Key%20Structure :default "None"))
  ;[0 0 0 0.5 32] AC_Health_Posture
  ;;[0.15 0.1244 0 0.5] Debug Take Posture Damage
  (:Pressed
    (Default|TakeDamage (Variables|Default|GetAC_Health_Posture) 0.0 4.0)))

(event Input|KeyboardEvents|2
  (params (Key :type Key%20Structure :default "None"))
  ;[0 0 0 0.5 32] AC_Health_Posture
  ;;[0.15 0.1244 0 0.5] Debug Take Health Damage
  (:Pressed
    (Default|TakeDamage (Variables|Default|GetAC_Health_Posture) 4.0 0.0)))

(event Input|KeyboardEvents|F
  (params (Key :type Key%20Structure :default "None"))
  ;[0 0 0 0.5 32] AC_Health_Posture
  ;;[0.15 0.1244 0 0.5] Debug Can Regen Posture
  (:Pressed
    (Variables|Default|SetCanRegenPosture (not (Variables|Default|GetCanRegenPosture)))))

(fn ConstructionScript)

(fn CameraLock
  (params (DeltaTime :type Float%20%28single-precision%29) (Target :type Vector%20%28by%20ref%29))
  (bind _returnvalue (Transformation|GetActorLocation))
  (bind _returnvalue_2 (Pawn|GetController))
  (bind _returnvalue_3 (Math|Rotator|FindLookatRotation _returnvalue Target))
  (bind _returnvalue_4 (Pawn|GetControlRotation _returnvalue_2 :!class /Script/Engine.Controller))
  (bind (_roll _pitch _yaw) (Math|Rotator|BreakRotator _returnvalue_3))
  (Utilities|FlowControl|Sequence
    (:then_0
      ;[0.15 0.15 0.15 0.5] Set the camera rotation to target
      (Pawn|SetControlRotation _returnvalue_2 (Math|Interpolation|RInterpTo _returnvalue_4 (Math|Rotator|MakeRotator (.Roll (Math|Rotator|BreakRotator _returnvalue_4)) _pitch _yaw) DeltaTime 4e+01)))
    (:then_1
      ;[0.15 0.15 0.15 0.5] Set Player rotation around target
      (Transformation|SetActorRotation (Math|Rotator|MakeRotator 0.0 0.0 (.yaw (Math|Interpolation|RInterpTo (Transformation|GetActorRotation) (Math|Rotator|FindLookatRotation (Transformation|GetActorLocation) Target) DeltaTime 25.0)))))))

(fn DecreasePosture
  (params (Delta%20Time :type Float%20%28double-precision%29))
  (bind _ac_health_posture (Variables|Default|GetAC_Health_Posture))
  (bind _ac_health_posture_2 (Variables|Default|GetAC_Health_Posture))
  (bind _currenthealth (Variables|/Game/Blueprints/ActorComponents/AC_Health_Posture.AC_Health_Posture_C|GetCurrentHealth _ac_health_posture_2))
  (bind _maxhealth (Variables|/Game/Blueprints/ActorComponents/AC_Health_Posture.AC_Health_Posture_C|GetMaxHealth _ac_health_posture_2))
  (bind _returnvalue (/ _currenthealth _maxhealth))
  ;[0.15 0.15 0.15 0.5] Posture Chart in Document
  (if (Variables|Default|GetCanRegenPosture)
    (if (Variables|Default|GetIsPlayerBlocking)
      (Default|TakeDamage _ac_health_posture 0.0 (* -2e+01 Delta%20Time))
      (elif (>= _returnvalue 0.75)
        (Default|TakeDamage _ac_health_posture 0.0 (* -13.3 Delta%20Time))
        (elif (>= _returnvalue 0.5)
          (Default|TakeDamage _ac_health_posture 0.0 (* -1e+01 Delta%20Time))
          (elif (>= _returnvalue 0.25)
            (Default|TakeDamage _ac_health_posture 0.0 (* -6.7 Delta%20Time))
            (else
              (Default|TakeDamage _ac_health_posture 0.0 (* -3.4 Delta%20Time)))))))))