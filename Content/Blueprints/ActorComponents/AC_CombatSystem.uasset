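; Actor component that gives a Character a melee combo attack system.
; TriggerAttack plays the current montage from an attack array and advances the index, wrapping at the end and resetting on completion.
; A "Combo Input Window" montage notify opens and closes CanAttack so attacks can chain.
; TriggerSimpleHit runs a forward box trace sized by an attack profile with debug drawing, but does not yet use the hit results.
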(event Custom|Trigger%20Attack
  (Variables|Default|GetCanAttack
    (:then
      (Variables|Default|SetCanAttack false)
      (bind _notifyname (Animation|Montage|PlayMontage (Variables|Default|GetMesh) (Utilities|Array|Get(acopy) (Variables|SystemParameters|GetAttackAnims) (Variables|SystemParameters|GetAttackIndexCurrent)))
        (:then
          (Variables|SystemParameters|SetAttackIndexCurrent (Math|Integer|SelectInt (+ (Variables|SystemParameters|GetAttackIndexCurrent) 1) 0 (< (Variables|SystemParameters|GetAttackIndexCurrent) (Utilities|Array|LastIndex (Variables|SystemParameters|GetAttackAnims))))))
        (:OnCompleted
          (Variables|Default|SetCanAttack true)
          (Variables|SystemParameters|SetAttackIndexCurrent 0))
        (:OnNotifyBegin
          ;[0.15 0.15 0.15 0.5] Allow player to string attacks in window (Case Senstaive)
          (switch name _notifyname
            (:ComboInputWindow
              (Variables|Default|SetCanAttack true))))
        (:OnNotifyEnd
          ;[0.15 0.15 0.15 0.5] Allow Recovery animation to play
          (switch name _notifyname
            (:ComboInputWindow
              (Variables|Default|SetCanAttack false))))))
    (:else)))

(event Custom|TriggerSimpleHit
  (params (AttackProfile :type F%20Attack%20Profile%20Structure))
  (bind _as_character (Variables|Default|GetAs%20Character))
  (bind _returnvalue (Transformation|GetActorLocation _as_character))
  (Class|KismetSystemLibrary|BoxTraceMultiforObjects _returnvalue (+ _returnvalue (* (Transformation|GetActorForwardVector _as_character) (.range AttackProfile))) (Math|Vector|MakeVector 0.0 (/ (.hitboxwidth AttackProfile) 2.0) (/ (.hitboxheight AttackProfile) 2.0)) (Transformation|GetActorRotation _as_character) (.hitableobjecttypes AttackProfile) false 0 "ForDuration" true))

(event EventBeginPlay
  (bind _ascharacter (Utilities|Casting|CastToCharacter (Components|GetOwner)))
  (Variables|Default|SetAs%20Character _ascharacter)
  (Variables|Default|SetMesh (Variables|/Script/Engine.Character|GetMesh _ascharacter)))

(event EventTick
  (params (DeltaSeconds :type Float%20%28single-precision%29)))