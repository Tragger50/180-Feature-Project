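; AC_Health_Posture is an actor component that tracks health and posture for its owning actor.
; A single TakeDamage event takes separate health and posture amounts, lowering health and building posture up, each clamped between zero and its maximum.
; It calls OnDeath when health reaches zero and OnPostureBreak when posture reaches its maximum.
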(event Custom|TakeDamage
  (params (HealthDamageAmount :type Float%20%28double-precision%29) (PostureDamageAmount :type Float%20%28double-precision%29))
  (Utilities|FlowControl|Sequence
    (:then_0
      ;[0.15 0.15 0.15 0.5] Take health Damage
      (bind _output_get (Variables|Default|SetCurrentHealth (Math|Float|Clamp(Float) (- (Variables|Default|GetCurrentHealth) HealthDamageAmount) 0.0 (Variables|Default|GetMaxHealth))))
      (if (<= _output_get 0.0)
        (Default|CallOnDeath)))
    (:then_1
      ;[0.15 0.15 0.15 0.5] Take posture Damage
      (bind _output_get_2 (Variables|Default|SetCurrentPosture (Math|Float|Clamp(Float) (+ (Variables|Default|GetCurrentPosture) PostureDamageAmount) 0.0 (Variables|Default|GetMaxPosture))))
      (if (>= _output_get_2 (Variables|Default|GetMaxPosture))
        (Default|CallOnPostureBreak)))))

(event EventBeginPlay)

(event EventTick
  (params (DeltaSeconds :type Float%20%28single-precision%29)))